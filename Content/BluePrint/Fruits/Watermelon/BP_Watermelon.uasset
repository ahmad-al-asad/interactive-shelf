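; BP_Watermelon is a watermelon fruit Blueprint with a Widget component that it shows, hides and rotates.
; Every Tick sets the Widget's visibility from the IsBoolean flag, without propagating to children.
; GetInstnaceFunction takes an Instance and turns the Widget's relative yaw 180 degrees opposite that Instance's RotationValue yaw, with roll and pitch zeroed.
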(event EventTick
  (params (DeltaSeconds :type Float%20%28single-precision%29))
  (bind _widget (Variables|Default|GetWidget))
  (if (Variables|Default|GetisBoolean)
    (Rendering|SetVisibility _widget true false)
    (else
      (Rendering|SetVisibility _widget false false))))

(fn ConstructionScript)

(fn GetInstnaceFunction
  (params (instance :type VR%20Pawn%20Object%20Reference))
  (bind _rotationvalue (Variables|/Game/VRTemplate/Blueprints/VRPawn.VRPawn_C|GetrotationValue instance))
  (bind _yaw (Math|Rotator|BreakRotator _rotationvalue))
  (Utilities|FlowControl|Sequence
    (:then_0
      (if (>= _yaw 1.8e+02)
        (Variables|Default|SetNewVar (- _yaw 1.8e+02))
        (else
          (Variables|Default|SetNewVar (+ _yaw 1.8e+02)))))
    (:then_1
      (Transformation|SetRelativeRotation (Variables|Default|GetWidget) (Math|Rotator|MakeRotator 0.0 0.0 (Variables|Default|GetNewVar)) false false))))